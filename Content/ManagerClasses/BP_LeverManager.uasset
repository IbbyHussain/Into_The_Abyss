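; BP_LeverManager is a manager actor that records the state of three levers as an array of booleans.
; Its UpdateboolArray event rebuilds BoolArray from the first three entries of LeverArray, storing the inverse of each lever's CanPullLever flag.
; The event only takes this snapshot; nothing in this Blueprint calls it or acts on the result.
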(event `self.UpdateboolArray`
  (set `self.boolArray` (`|MakeArray` (not (`C_BaseAnimLever.bCanPullLever` (`|GetArrayItem` (`self.LeverArray`)))) (not (`C_BaseAnimLever.bCanPullLever` (`|GetArrayItem` (`self.LeverArray`) 1))) (not (`C_BaseAnimLever.bCanPullLever` (`|GetArrayItem` (`self.LeverArray`) 2))))))

(fn `UserConstructionScript`)