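; Manager for the lab level that runs the timed ending sequence once the puzzles are complete, finishing by loading TheLab.
; PuzzlesAreComplete locks player movement and input, hides HUD souls and crosshair, then calls PlayCinematic.
; Chained delays then spawn a dummy black hole, play reaction montages on two scientists, trigger SpawnBlackHole and layer camera and black screen widgets.
; A separate ChangeLighting event calls ChangeLights.
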(event `self.PuzzlesAreComplete`
  (bind _returnvalue (`GameplayStatics.GetPlayerCharacter` 0))
  (bind _returnvalue_2 (`GameplayStatics.GetPlayerController` 0))
  (`CharacterMovementComponent.DisableMovement` (`Character.CharacterMovement` _returnvalue))
  (`self.DisableInput` _returnvalue _returnvalue_2)
  (bind _asbp_player_hud2 (cast `/Game/UI/BP_PlayerHUD2` (`PlayerController.GetHUD` _returnvalue_2)))
  (bind _aswbp_hudwidget_2 (cast `/Game/UI/WBP_HUDWidget2` (`C_PlayerHUD2.HUDWidget` _asbp_player_hud2)))
  (`/Game/UI/WBP_HUDWidget2.SetSoulsVisibility` _aswbp_hudwidget_2 "Hidden")
  (`/Game/UI/WBP_HUDWidget2.SetCrosshairVisibility` _aswbp_hudwidget_2 "Hidden")
  (`self.Play Cinematic`)
  (`KismetSystemLibrary.Delay` 16.75)
  (`|SpawnActorFromClass` "/Game/Enviroment/Scientist/BlackHole/BP_BlackHoleDummy.BP_BlackHoleDummy_C" (`KismetMathLibrary.MakeTransform` (`self.K2_GetActorLocation` (`self.DummyHoleSpawnLoc`))) "Undefined" "OverrideRootScale" null null)
  (`KismetSystemLibrary.Delay` 3.0)
  (`|PlayMontage` (`Character.Mesh` (`self.Scientist1`)) "/Game/AI/Scientists/Animations/BackgroundAnimations/LevelSequenceAnims/AM_Turn.AM_Turn"
    (:`then`
      (`|PlayMontage` (`Character.Mesh` (`self.Scientist2`)) "/Game/AI/Scientists/Animations/BackgroundAnimations/LevelSequenceAnims/AM_Terrified.AM_Terrified"
        (:`then`
          (`KismetSystemLibrary.Delay` 3.0)
          (`self.SpawnBlackHole`)
          (`KismetSystemLibrary.Delay` 2.75)
          (bind _returnvalue_3 (`|CreateWidget` "/Game/UI/MISC/WBP_Camera.WBP_Camera_C"))
          (`UserWidget.AddToViewport` _returnvalue_3 0)
          (`KismetSystemLibrary.Delay` 7.65)
          (bind _returnvalue_4 (`|CreateWidget` "/Game/UI/WBP_Black.WBP_Black_C"))
          (`UserWidget.AddToViewport` _returnvalue_4 0)
          (`GameplayStatics.OpenLevel` "TheLab"))))))

(event `self.ChangeLighting`
  (`self.Change Lights`))

(fn `UserConstructionScript`)