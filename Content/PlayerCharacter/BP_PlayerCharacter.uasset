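; Player character Blueprint that handles crossbow bolt cycling with the mouse wheel while in ranged combat.
; BeginPlay caches the time-swap and moveable-object managers and sets game-only input.
; Each scroll switches bolts, dummy bolts and bolt icons in sequence, each through its own next/previous evaluation.
; Tick is empty, F only toggles a bool, and disconnected test snippets for damage, wall spawning and hold timing remain.
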(event `self.ReceiveBeginPlay`
  ;[1 1 1] Sets Values of pointers
  (`|ExecutionSequence`
    (:`then_0`
      (bind _outactors (`GameplayStatics.GetAllActorsOfClass` "/Script/MyProject.TimeMechanicManagerClass"))
      (set `self.SwapTimeManager` (`|GetArrayItem` _outactors))
      (bind _outactors_2 (`GameplayStatics.GetAllActorsOfClass` "/Game/ManagerClasses/BP_MoveableObjectManager1.BP_MoveableObjectManager1_C"))
      (set `self.MoveableObjectManager` (`|GetArrayItem` _outactors_2))
      (`WidgetBlueprintLibrary.SetInputMode_GameOnly` (`GameplayStatics.GetPlayerController` 0)))))

(event `InputAxisKey|MouseWheelAxis`
  (params (AxisValue :type "Float (single-precision)"))
  (if (`|EnumEquality` (`self.CombatState`) "RANGED")
    (`|ExecutionSequence`
      (:`then_0`
        ;[1 1 1] Bolt Switching
        (`/Engine/EditorBlueprintResources/StandardMacros.CompareFloat` AxisValue
          (:`>`
            ;;[1 1 1] Next Bolt
            (bind _returnvalue (`self.EvaluateNextBolt`))
            (`self.SwitchBolts` _returnvalue))
          (:`<`
            ;;[1 1 1] Previous Bolt
            (bind _returnvalue_2 (`self.EvaluatePreviousBolt` (`KismetArrayLibrary.Array_LastIndex` (`C_Crossbow.BoltsArray` (`.CrossbowObject` (break `Crossbow` (`self.Crossbow`)))))))
            (`self.SwitchBolts` _returnvalue_2))))
      (:`then_1`
        ;[1 1 1] Dummy Bolt Switching
        (`/Engine/EditorBlueprintResources/StandardMacros.CompareFloat` AxisValue
          (:`>`
            ;;[1 1 1] Next Bolt
            (bind _returnvalue_3 (`self.EvaluateNextDummyBolt`))
            (`self.SwitchDummyBolts` _returnvalue_3))
          (:`<`
            ;;[1 1 1] Previous Bolt
            (bind _returnvalue_4 (`self.EvaluatePreviousDummyBolt` (`KismetArrayLibrary.Array_LastIndex` (`C_Crossbow.DummyBoltsArray` (`.CrossbowObject` (break `Crossbow` (`self.Crossbow`)))))))
            (`self.SwitchDummyBolts` _returnvalue_4))))
      (:`then_2`
        ;[1 1 1] Bolt Icon Switching
        (`/Engine/EditorBlueprintResources/StandardMacros.CompareFloat` AxisValue
          (:`>`
            ;;[1 1 1] Next Bolt
            (bind _returnvalue_5 (`self.EvaluateNextBoltIcon`))
            (`self.SwitchBoltIcon` _returnvalue_5))
          (:`<`
            ;;[1 1 1] Previous Bolt
            (bind _returnvalue_6 (`self.EvaluatePreviousBoltIcon` (`KismetArrayLibrary.Array_LastIndex` (`C_Crossbow.BoltIconArray` (`.CrossbowObject` (break `Crossbow` (`self.Crossbow`)))))))
            (`self.SwitchBoltIcon` _returnvalue_6)))))))

(event `Key|G`
  (params (Key :type "Key Structure"))
  ;[1 1 1] Algorithm for last time this event was called
)

(event `self.ReceiveTick`
  (params (DeltaSeconds :type "Float (single-precision)")))

(event `Key|F`
  (params (Key :type "Key Structure"))
  (:`Pressed`
    (set `self.bool` true))
  (:`Released`
    (set `self.bool` false)))

(event `Key|G`
  (params (Key :type "Key Structure")))

(fn `UserConstructionScript`)