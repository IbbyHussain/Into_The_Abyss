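; BP_StructuralSupport is a mine shaft environment Blueprint that places structural support meshes as instances.
; The construction script loops over InstanceLocationArray and adds a Hierarchical Instanced Static Mesh instance per entry, keeping its rotation, halving its location and forcing unit scale.
; BeginPlay is empty, and the Event Graph holds an unconnected, nested-loop version of the same placement logic that never runs.
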(event `self.ReceiveBeginPlay`)

(fn `UserConstructionScript`
  (for _array_element (`self.Instance Location Array`)
    (`InstancedStaticMeshComponent.AddInstance` (`self.HierarchicalInstancedStaticMesh`) (`KismetMathLibrary.MakeTransform` (/ (.location _array_element) 2.0) (.rotation _array_element)))))