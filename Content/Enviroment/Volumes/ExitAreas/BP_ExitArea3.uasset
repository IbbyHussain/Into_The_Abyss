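; BP_ExitArea3 is an exit area volume that responds when the player presses E inside it.
; BeginPlay stores a hardcoded exit area location.
; Tick polls the player capsule's overlap with the box and the character's CanExit and EKeyPressed flags.
; When all hold, it waits through a Delay, calls EKeyPressed, defined outside these graphs, then hides the HUD's E-key hint.
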(event `self.ReceiveBeginPlay`
  (set `self.ExitAreaActorLocation` (500.0 2000.0 150.0)))

(event `self.ReceiveTick`
  (params (DeltaSeconds :type "Float (single-precision)"))
  (if (`PrimitiveComponent.IsOverlappingComponent` (`Character.CapsuleComponent` (`GameplayStatics.GetPlayerCharacter` 0)) (`self.BoxComp`))
    (bind _asbp_player_character (cast `/Game/PlayerCharacter/BP_PlayerCharacter` (`GameplayStatics.GetPlayerCharacter` 0)))
    (if (and (`C_PlayerCharacter.bCanExit` _asbp_player_character) (`C_PlayerCharacter.bEKeyPressed` _asbp_player_character))
      (`KismetSystemLibrary.Delay` 2.0)
      (`self.EKeyPressed`)
      (bind _asbp_player_hud2 (cast `/Game/UI/BP_PlayerHUD2` (`PlayerController.GetHUD` (`GameplayStatics.GetPlayerController` 0))))
      (`C_PlayerHUD2.EKeyHintInVisible` _asbp_player_hud2))))

(fn `UserConstructionScript`)