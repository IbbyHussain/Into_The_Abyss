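; BP_ExitArea1 is an exit volume that teleports the player character to a stored location when the E key is pressed inside it.
; Tick polls whether the player's capsule overlaps the box component, printing a debug message, and reads the key state from BP_PlayerCharacter.
; After a short delay it moves the character to Loc without sweeping, then hides the E key hint through BP_PlayerHUD2.
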(event `self.ReceiveTick`
  (params (DeltaSeconds :type "Float (single-precision)"))
  (if (`PrimitiveComponent.IsOverlappingComponent` (`Character.CapsuleComponent` (`GameplayStatics.GetPlayerCharacter` 0)) (`self.BoxComp`))
    (`KismetSystemLibrary.PrintString` "OverLapping" true true (struct :`G` 0.66 :`B` 1.0 :`A` 1.0) 1.0)
    (bind _asbp_player_character (cast `/Game/PlayerCharacter/BP_PlayerCharacter` (`GameplayStatics.GetPlayerCharacter` 0)))
    (if (`C_PlayerCharacter.bEKeyPressed` _asbp_player_character)
      (`KismetSystemLibrary.Delay` 2.0)
      (`self.K2_SetActorLocation` _asbp_player_character (`self.Loc`) false false)
      (bind _asbp_player_hud2 (cast `/Game/UI/BP_PlayerHUD2` (`PlayerController.GetHUD` (`GameplayStatics.GetPlayerController` 0))))
      (`C_PlayerHUD2.EKeyHintInVisible` _asbp_player_hud2))))

(fn `UserConstructionScript`)