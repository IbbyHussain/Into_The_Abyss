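; AC_POI is an actor component that places a point-of-interest marker for its owner on the HUD minimap.
; Shortly after BeginPlay it finds the WBP_HUDWidget2 widget, calls AddPOI on its MiniMap and stores the returned marker.
; For BP_NPC_Scientist owners, it hides the marker if the NPC should not have a quest icon.
; Tick also polls that NPC's quest and hides the marker once completed.
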(event `self.ReceiveBeginPlay`
  (`KismetSystemLibrary.Delay` 0.2)
  (`self.Owner`
    (:`then`
      (`|ExecutionSequence`
        (:`then_0`
          (bind _foundwidgets (`WidgetBlueprintLibrary.GetAllWidgetsOfClass` "/Game/UI/WBP_HUDWidget2.WBP_HUDWidget2_C"))
          (bind _aswbp_hudwidget_2 (cast `/Game/UI/WBP_HUDWidget2` (`|GetArrayItem` _foundwidgets)))
          (bind _returnvalue (`C_MiniMap.AddPOI` (`/Game/UI/WBP_HUDWidget2.MiniMap` _aswbp_hudwidget_2) (`self.Owner`)))
          (set `self.POI` _returnvalue)
          (bind _asbp_npc_scientist (cast `/Game/AI/NPCs/BP_NPC_Scientist` (`self.Owner`)))
          (set `self.QuestNPC` _asbp_npc_scientist))
        (:`then_1`
          (bind _questnpc (`self.QuestNPC`)
            (:`then`
              (if (not (`C_QuestNPC.bShouldHaveQuestIcon` _questnpc))
                (bind _poi (`self.POI`)
                  (:`then`
                    (`Widget.SetVisibility` _poi "Hidden"))
                  (:`else`))))
            (:`else`)))))
    (:`else`)))

(event `self.ReceiveTick`
  (params (DeltaSeconds :type "Float (single-precision)"))
  (bind _questnpc (`self.QuestNPC`)
    (:`then`
      (bind _questref (`C_QuestNPC.QuestREF` _questnpc)
        (:`then`
          (if (`C_BaseQuest.bIsCompleted` _questref)
            (bind _poi (`self.POI`)
              (:`then`
                (`Widget.SetVisibility` _poi "Hidden"))
              (:`else`))))
        (:`else`)))
    (:`else`)))