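; Scientist NPC that displays available-quest markers and wears an optional backpack and a helmet that can be hidden.
; BeginPlay sets the quest image on front and back widgets, calls DestroyQuestWidgets, registers itself as POI owner, applies the cloth-simulation setting and spawns gear on sockets.
; Tick polls both markers against the assigned quest and calls DestroyQuestWidgets once it is completed.
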(event `self.ReceiveBeginPlay`
  (`|ExecutionSequence`
    (:`then_0`
      (bind _aswbp_available_quest (cast `/Game/Quest_System/Quest_UI/WBP_AvailableQuest` (`WidgetComponent.GetUserWidgetObject` (`self.FrontQuestWidget`))))
      (set `self.WBP_AvailableQuestREF` _aswbp_available_quest)
      (bind _aswbp_available_quest_2 (cast `/Game/Quest_System/Quest_UI/WBP_AvailableQuest` (`WidgetComponent.GetUserWidgetObject` (`self.BackQuestWidget`))))
      (set `self.WBP_AvailableQuestREF2` _aswbp_available_quest_2)
      (`C_AvailableQuest.SetQuestMarkerImage` _aswbp_available_quest (`self.QuestREF`))
      (`C_AvailableQuest.SetQuestMarkerImage` _aswbp_available_quest_2 (`self.QuestREF`)))
    (:`then_1`
      (`self.DestroyQuestWidgets` true)
      (set `C_POIComponent.Owner` self (`self.AC_POI`))
      (set `SkeletalMeshComponent.bDisableClothSimulation` (`self.Disable Cloth`) (`self.Mesh`))
      (bind _returnvalue (`self.SpawnItem` "HelmSocket" (`self.Helmptr`) true (`self.Helm Class`)))
      (`|ExecutionSequence`
        (:`then_0`
          (if (`self.bShouldHaveBackpack`)
            (`self.SpawnItem` "BackpackSocket" (`self.Backpackptr`) true "/Game/AI/Scientists/BP_ScientistBackpack.BP_ScientistBackpack_C")))
        (:`then_1`
          (if (`self.ShouldHelmBeInVisible`)
            (`self.SetActorHiddenInGame` _returnvalue true)))))))

(event `self.ReceiveTick`
  (params (DeltaSeconds :type "Float (single-precision)"))
  (`C_AvailableQuest.CheckQuestMarkerImage` (`self.WBP_AvailableQuestREF`) (`self.QuestREF`))
  (`C_AvailableQuest.CheckQuestMarkerImage` (`self.WBP_AvailableQuestREF2`) (`self.QuestREF`))
  (if (`C_BaseQuest.bIsCompleted` (`self.QuestREF`))
    (`self.DestroyQuestWidgets` false)))

(fn `UserConstructionScript`)