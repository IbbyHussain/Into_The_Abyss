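; Test Behavior Tree task for melee AI that picks a location near player 0 and prepares the pawn's movement.
; It writes a random navigable point to the Blackboard, offset by Distance from the player within a cone facing the pawn.
; It then sets walk speed and focuses the controller on the player if a debug-drawn Camera trace hits them.
; The task finishes immediately without moving the pawn itself.
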(event `self.ReceiveExecuteAI`
  (params (OwnerController :type "AIController Object Reference") (ControlledPawn :type "Pawn Object Reference"))
  (set `self.Controller` OwnerController)
  (set `self.Pawn` ControlledPawn)
  (`BTFunctionLibrary.SetBlackboardValueAsVector` (`self.BB Target loc`) (`NavigationSystemV1.K2_GetRandomLocationInNavigableRadius` (+ (`Actor.K2_GetActorLocation` (`GameplayStatics.GetPlayerCharacter` 0)) (* (`KismetMathLibrary.RandomUnitVectorInConeInDegrees` (`KismetMathLibrary.GetDirectionUnitVector` (`Actor.K2_GetActorLocation` (`GameplayStatics.GetPlayerCharacter` 0)) (`Actor.K2_GetActorLocation` ControlledPawn)) 60.0) (`self.distance`))) 50.0 null null))
  (`self.Walk speed func`)
  (`self.Focus func`)
  (`self.FinishExecute` true))

(fn `Focus func`
  (bind _pawn (`self.Pawn`))
  (bind _outhit (`KismetSystemLibrary.LineTraceSingle` (`Actor.K2_GetActorLocation` _pawn) (`Actor.K2_GetActorLocation` (`GameplayStatics.GetPlayerCharacter` 0)) "TraceTypeQuery2" false (`|MakeArray` _pawn :!type "Actor Object Reference") "ForDuration"))
  (if (== (`.HitActor` (`GameplayStatics.BreakHitResult` _outhit)) (`GameplayStatics.GetPlayerCharacter` 0))
    (`AIController.K2_SetFocus` (`self.Controller`) (`.HitActor` (`GameplayStatics.BreakHitResult` _outhit)))))

(fn `Walk speed func`
  (bind _ascharacter (cast `Character` (`self.Pawn`)))
  (set `CharacterMovementComponent.MaxWalkSpeed` (`self.Walk speed`) (`Character.CharacterMovement` _ascharacter)))