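; AI controller for the savage melee enemy that tracks whether it perceives the player.
; When AI perception updates on a BP_PlayerCharacter, it writes the sensed result to the BPCanSeePlayer blackboard key.
; It also copies that same value straight into the player's IsHidden variable, so IsHidden is true while the player is sensed.
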(event `self.AIPerception.OnTargetPerceptionUpdated`
  (params (Actor :type "Actor Object Reference") (Stimulus :type "AIStimulus Structure"))
  (bind (_age _expirationage _strength _stimuluslocation _receiverlocation _tag _bsuccessfullysensed) (break `AIStimulus` Stimulus))
  (bind _asbp_player_character (cast `/Game/PlayerCharacter/BP_PlayerCharacter` Actor))
  (`|ExecutionSequence`
    (:`then_0`
      (`BlackboardComponent.SetValueAsBool` (`AIBlueprintHelperLibrary.GetBlackboard` null) "BPCanSeePlayer" _bsuccessfullysensed)
      (set `C_PlayerCharacter.bIsHidden` _bsuccessfullysensed _asbp_player_character))))

(fn `UserConstructionScript`)