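; Manager for melee AI fights that ranks enemies by grade and periodically picks the top one, apparently for attack turns.
; On BeginPlay it gives each AI in AIArray a random starting grade in AIMap and attaches a debug widget showing it.
; A looping timer grades by location, resets the highest-graded AI and refreshes affected widgets.
; No attack command is issued in these graphs, and GenerateMapElements is unwired.
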(event `self.ReceiveBeginPlay`
  (for _array_element (`self.AIArray`)
    (`BlueprintMapLibrary.Map_Add` (`self.AIMap`) _array_element (`KismetMathLibrary.RandomFloatInRange` 1.0 5.0))
    (bind _returnvalue (`|CreateWidget` "/Game/AI/Base_MeleeAI/WBP_DebugMeleeAI.WBP_DebugMeleeAI_C" null (`BlueprintMapLibrary.Map_Find` (`self.AIMap`) _array_element) _array_element))
    (`BlueprintMapLibrary.Map_Add` (`self.Enemy Widgets`) _array_element _returnvalue)
    (bind _returnvalue_2 (`AddComponent|NODE_AddWidgetComponent-1` :`self` _array_element))
    (`WidgetComponent.SetWidget` _returnvalue_2 _returnvalue))
  (`KismetSystemLibrary.K2_SetTimerDelegate` (delegate `trigger attack`) 8.0 true))

(event `trigger attack`
  (bind _returnvalue (`self.GradeByLocation`))
  (set `/Game/AI/Base_MeleeAI/WBP_DebugMeleeAI.Grade` (`BlueprintMapLibrary.Map_Find` (`self.AIMap`) _returnvalue) (`BlueprintMapLibrary.Map_Find` (`self.Enemy Widgets`) _returnvalue))
  (bind (_newlocalvar_01 _newlocalvar_12) (`self.Evaluate AI Grades `))
  (`self.ResetAIGrade` _newlocalvar_12)
  (set `/Game/AI/Base_MeleeAI/WBP_DebugMeleeAI.Grade` (`BlueprintMapLibrary.Map_Find` (`self.AIMap`) _newlocalvar_12) (`BlueprintMapLibrary.Map_Find` (`self.Enemy Widgets`) _newlocalvar_12)))

(fn `Evaluate AI Grades `
  (returns (NewLocalVar_01 :type "Float (double-precision)") (NewLocalVar_12 :type "C_MeleeAI Object Reference"))
  (locals (NewLocalVar_0 :type "Float (double-precision)") (NewLocalVar_1 :type "C_MeleeAI Object Reference"))
  (bind _keys (`BlueprintMapLibrary.Map_Keys` (`self.AIMap`)))
  (for _array_element _keys
    (bind _value (`BlueprintMapLibrary.Map_Find` (`self.AIMap`) _array_element))
    (if (> _value (`local.NewLocalVar_0`))
      (set `local.NewLocalVar_0` _value)
      (set `local.NewLocalVar_1` _array_element)))
  (return (`local.NewLocalVar_0`) (`local.NewLocalVar_1`)))

(fn `UserConstructionScript`)