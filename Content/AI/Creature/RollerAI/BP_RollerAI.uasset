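; BP_RollerAI is a creature Blueprint whose graph only cycles the colour of its mesh; no movement or AI logic appears here.
; On BeginPlay it creates a dynamic material instance, stores the starting Colour parameter and starts a looping timer.
; Each timer tick picks a random colour and plays a timeline that lerps the parameter to it.
; When the timeline finishes, that colour becomes the next blend's start.
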(event `self.ReceiveBeginPlay`
  (bind _meshcomp (`self.MeshComp`))
  (bind _returnvalue (`PrimitiveComponent.CreateDynamicMaterialInstance` _meshcomp 0 (`|GetArrayItem` (`MeshComponent.GetMaterials` _meshcomp)) "None"))
  (bind _output_get (set `self.DynamicMaterial` _returnvalue))
  (bind _returnvalue_2 (`MaterialInstanceDynamic.K2_GetVectorParameterValue` _output_get "Colour"))
  (set `self.Init Colour` _returnvalue_2)
  (`KismetSystemLibrary.K2_SetTimerDelegate` (delegate `CustomEvent_0`) 2.0 true))

(event `CustomEvent_0`
  (set `self.New Colour` (`KismetMathLibrary.MakeColor` (`KismetMathLibrary.RandomFloatInRange` 0.0 1.0) (`KismetMathLibrary.RandomFloatInRange` 0.0 1.0) (`KismetMathLibrary.RandomFloatInRange` 0.0 1.0) 0.0))
  (bind (_direction _newtrack_0) (`Timeline|Chnage colour timeline` :!via `PlayFromStart`)
    (:`Update`
      (`MaterialInstanceDynamic.SetVectorParameterValue` (`self.DynamicMaterial`) "Colour" (`KismetMathLibrary.LinearColorLerp` (`self.Init Colour`) (`self.New Colour`) _newtrack_0)))
    (:`Finished`
      (set `self.Init Colour` (`self.New Colour`)))))

(fn `UserConstructionScript`)