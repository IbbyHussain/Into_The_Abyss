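; Purple larva projectile for the Summoner boss that damages the player or the player's mud wall.
; When not flagged as a player bolt, its Box overlap calls the player's damage function, with a flag limiting this to one hit.
; Hitting the mud wall referenced by the player character applies generic damage and destroys the projectile, while a player hit leaves it alive.
; Both hit branches print debug strings.
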(event `self.Box.OnComponentBeginOverlap`
  (params (OverlappedComponent :type "PrimitiveComponent Object Reference") (OtherActor :type "Actor Object Reference") (OtherComp :type "PrimitiveComponent Object Reference") (OtherBodyIndex :type Integer) (bFromSweep :type Boolean) (SweepResult :type "HitResult Structure (by ref)"))
  (bind _returnvalue (`GameplayStatics.GetPlayerCharacter` 0))
  (if (`self.bIsPlayerBolt`)
    _
    (elif (== OtherActor _returnvalue)
      (bind _asbp_player_character (cast `/Game/PlayerCharacter/BP_PlayerCharacter` _returnvalue))
      (if (not (`self.bHasOverlapped`))
        (set `self.bHasOverlapped` true)
        (`C_PlayerCharacter.ApplyDamageToPlayer` _asbp_player_character 10.0)
        (`KismetSystemLibrary.PrintString` "PLAYER"))
      (else
        (bind _asbp_player_character_2 (cast `/Game/PlayerCharacter/BP_PlayerCharacter` _returnvalue))
        (bind _mudwallactor (`C_PlayerCharacter.MudWallActor` _asbp_player_character_2))
        (if (== _mudwallactor OtherActor)
          (`GameplayStatics.ApplyDamage` _mudwallactor 1.0)
          (`KismetSystemLibrary.PrintString` "WALL")
          (`self.K2_DestroyActor`))))))

(fn `UserConstructionScript`)