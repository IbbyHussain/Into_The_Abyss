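; BP_PeasantAI is an English peasant AI that randomizes its equipment at BeginPlay.
; It spawns one of three weapons (brute axe, pickaxe or sickle) and either a mining backpack, a regular backpack or none.
; References to both spawned items are stored so DestroyAIItems can destroy whichever are still valid.
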(event `self.ReceiveBeginPlay`
  ;[1 1 1] Spawning of objects
  (bind _returnvalue (`self.SpawnWeapon` (`|GetArrayItem` (`|MakeArray` "/Game/AI/English/Brute/Brute_Accessories/Brute_Axe/BP_BruteAxe.BP_BruteAxe_C" "/Game/AI/English/Peasant/Peasant_Accessories/Pickaxe/BP_PeasantPickaxe.BP_PeasantPickaxe_C" "/Game/AI/English/Peasant/Peasant_Accessories/Sickle/BP_PeasantSickle.BP_PeasantSickle_C" :!type "Actor Class Reference") (`KismetMathLibrary.RandomInteger` 3)) "/Game/AI/English/Peasant/Peasant_Accessories/Sickle/BP_PeasantSickle.BP_PeasantSickle_C"))
  (set `self.Weapon PTR` _returnvalue)
  (bind _returnvalue_2 (`self.SpawnBackpack` (`|GetArrayItem` (`|MakeArray` "/Game/AI/English/Peasant/Peasant_Accessories/BackPack/Mining_Backpack/BP_Mining_Backpack.BP_Mining_Backpack_C" "/Game/AI/English/Peasant/Peasant_Accessories/BackPack/Default_Backpack/BP_Backpack.BP_Backpack_C" null :!type "C_SkeletalMeshActor Class Reference") (`KismetMathLibrary.RandomInteger` 3))))
  (set `self.Backpack PTR` _returnvalue_2))

(event `self.DestroyAIItems`
  (bind _weapon_ptr (`self.Weapon PTR`))
  (bind _backpack_ptr (`self.Backpack PTR`))
  (`|ExecutionSequence`
    (:`then_0`
      (if (`KismetSystemLibrary.IsValid` _weapon_ptr)
        (`self.K2_DestroyActor` _weapon_ptr)))
    (:`then_1`
      (if (`KismetSystemLibrary.IsValid` _backpack_ptr)
        (`self.K2_DestroyActor` _backpack_ptr)))))

(fn `UserConstructionScript`)