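; BP_Savage is the Savage enemy AI Blueprint, armed with a randomly chosen two-handed weapon.
; On BeginPlay it picks the axe, sword or scythe class, spawns it through SpawnTwoHandedWeapon and stores the result in WeaponPTR.
; DestroyAIItems destroys that weapon if it is still valid.
; Two small functions forward restart-attack and test calls to BPFightManager.
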(event `self.ReceiveBeginPlay`
  ;[1 1 1] Spawning of objects
  (bind _returnvalue (`self.SpawnTwoHandedWeapon` (`|GetArrayItem` (`|MakeArray` "/Game/AI/English/Savage/Savage_Accessories/Savage_Axe/BP_SavageAxe.BP_SavageAxe_C" "/Game/AI/English/Savage/Savage_Accessories/Savage_Sword/BP_SavageSword.BP_SavageSword_C" "/Game/AI/English/Savage/Savage_Accessories/Savage_Scythe/BP_SavageScythe.BP_SavageScythe_C" :!type "Actor Class Reference") (`KismetMathLibrary.RandomInteger` 3)) "/Game/AI/English/Savage/Savage_Accessories/Savage_Sword/BP_SavageSword.BP_SavageSword_C"))
  (set `self.Weapon PTR` _returnvalue))

(event `self.DestroyAIItems`
  (bind _weapon_ptr (`self.Weapon PTR`))
  (if (`KismetSystemLibrary.IsValid` _weapon_ptr)
    (`self.K2_DestroyActor` _weapon_ptr)))

(fn `Call Fight Manager Restart Attack`
  (`/Game/AI/Base_MeleeAI/BP_AIFightManager.restart attack` (`self.BP_fight manager`)))

(fn `call fight manager test`
  (`/Game/AI/Base_MeleeAI/BP_AIFightManager.test` (`self.BP_fight manager`)))

(fn `UserConstructionScript`)